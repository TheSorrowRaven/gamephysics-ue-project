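; Base weapon actor that players can pick up, drop and fire, with magazine ammo shown on a text display.
; Shoot checks a Tick-driven cooldown and ammo, then line-traces from the muzzle with random recoil spread that grows per shot and recovers over time.
; The trace result feeds SpawnProjectile, an empty hook for child weapons.
; Helpers deal damage through I_Damageable and report hits to the PlayerCharacter.
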(event EventBeginPlay
  (CallFunction|UpdateAmmoDisplay))

(event EventTick
  (params (DeltaSeconds :type Float%20%28single-precision%29))
  (Variables|Default|SetShoot_RateCooldown (- (Variables|Default|GetShoot_RateCooldown) DeltaSeconds))
  (CallFunction|UpdateRecoil DeltaSeconds))

(fn ConstructionScript)

(fn CanShoot
  (bind _has_ammo (CallFunction|HasAmmoinMagazine))
  (if _has_ammo
    (if (< (Variables|Default|GetShoot_RateCooldown) 0.0)
      (return true)
      (else
        _)))
  (return false))

(fn HasAmmoinMagazine
  (return (> (Variables|Default|GetAmmo_MagazineAmount) 0)))

(fn ShootRateZero
  (if (< (Variables|Default|GetShoot_RateCooldown) 0.0)
    (return true)
    (else
      (return false))))

(fn Shoot
  (params (Instigator :type Base%20Character%20Object%20Reference))
  (bind _shoot_rate_zero (CallFunction|ShootRateZero))
  (if _shoot_rate_zero
    (bind _has_ammo (CallFunction|HasAmmoinMagazine))
    (if _has_ammo
      (CallFunction|ActuallyShoot Instigator)
      (return true)
      (else
        (Audio|PlaySoundatLocation "/Game/3rdParty/Audio/Sounds/weapon_outOfAmmo.weapon_outOfAmmo" (Transformation|GetActorLocation) "0, 0, 0" 1.0 1.0 0.0 0 0 0)
        (CallFunction|ResetShootRate)
        (return false)))
    (else
      (return false))))

(fn ActuallyShoot
  (params (Instigator :type Base%20Character%20Object%20Reference))
  (bind _mesh (Variables|Default|GetMesh))
  (bind _returnvalue (Transformation|GetSocketLocation _mesh "Muzzle"))
  (bind _rotator (CallFunction|GetRecoil))
  (bind _outhit (Collision|LineTraceByChannel _returnvalue (+ _returnvalue (* (Math|Vector|RotateVector (Math|Vector|GetForwardVector (Variables|Default|GetMesh)) _rotator) 1e+04)) "TraceTypeQuery3" false 0 "None"))
  (CallFunction|SpawnProjectile Instigator _returnvalue (select (.bBlockingHit (Collision|BreakHitResult _outhit)) (.Location (Collision|BreakHitResult _outhit)) (+ _returnvalue (* (Math|Vector|RotateVector (Math|Vector|GetForwardVector (Variables|Default|GetMesh)) _rotator) 1e+04))) (.Normal (Collision|BreakHitResult _outhit)) (.HitActor (Collision|BreakHitResult _outhit)))
  (CallFunction|ResetShootRate)
  (CallFunction|AddRecoil)
  (Audio|PlaySoundatLocation (Variables|Default|GetSound_Shoot) (Transformation|GetActorLocation self) "0, 0, 0" 1.0 1.0 0.0 0 0 0)
  (CallFunction|RemoveAmmo 1))

(fn SpawnProjectile
  (params (Instigator :type Base%20Character%20Object%20Reference) (FromLocation :type Vector) (ToLocation :type Vector) (HitNormal :type Vector) (HitActor :type Actor%20Object%20Reference) (Bounce%20Count :type Integer)))

(fn AddAmmo
  (params (Amount :type Integer))
  (if (< (Variables|Default|GetAmmo_MagazineAmount) (Variables|Default|GetAmmo_MagazineSize))
    (if (<= (- (+ (Variables|Default|GetAmmo_MagazineAmount) Amount) (Variables|Default|GetAmmo_MagazineSize)) 0)
      (Variables|Default|SetAmmo_MagazineAmount (+ (Variables|Default|GetAmmo_MagazineAmount) Amount))
      (CallFunction|UpdateAmmoDisplay)
      (return 0)
      (else
        (Variables|Default|SetAmmo_MagazineAmount (Variables|Default|GetAmmo_MagazineSize))
        (CallFunction|UpdateAmmoDisplay)
        (return (- (+ (Variables|Default|GetAmmo_MagazineAmount) Amount) (Variables|Default|GetAmmo_MagazineSize)))))
    (else
      (return Amount))))

(fn RemoveAmmo
  (params (Amount :type Integer))
  (Variables|Default|SetAmmo_MagazineAmount (- (Variables|Default|GetAmmo_MagazineAmount) Amount))
  (CallFunction|UpdateAmmoDisplay))

(fn PickUp
  (params (Holder :type Base%20Character%20Object%20Reference))
  (bind _can_pick_up (CallFunction|CanPickUp))
  (if _can_pick_up
    (Variables|Default|SetHolder Holder)
    (Physics|SetSimulatePhysics (Variables|Default|GetMesh) false)
    (Collision|SetCollisionEnabled (Variables|Default|GetMesh) "NoCollision")
    (else
      (Development|PrintString "Already Picked Up!"))))

(fn CanPickUp
  (if (== (Variables|Default|GetHolder) 0)
    (return true)
    (else
      (return false))))

(fn DropWeapon
  (Transformation|DetachFromActor "KeepWorld" "KeepWorld" "KeepWorld")
  (Variables|Default|SetHolder 0)
  (Physics|SetSimulatePhysics (Variables|Default|GetMesh) true)
  (Collision|SetCollisionEnabled (Variables|Default|GetMesh) "QueryAndPhysics"))

(fn UpdateAmmoDisplay
  (Rendering|Components|TextRender|SetText (Variables|Default|GetAmmo%20Text) (Utilities|Text|ToText(Integer) (Variables|Default|GetAmmo_MagazineAmount))))

(fn ResetShootRate
  (Variables|Default|SetShoot_RateCooldown (Variables|Default|GetShoot_Rate)))

(fn DealDamage
  (params (Damage%20Actor :type Actor%20Object%20Reference) (Hit%20Location :type Vector))
  (bind _asi_damageable (Utilities|Casting|CastToI_Damageable Damage%20Actor)
    (:then
      (bind _receiver_died (Default|ReceiveDamage _asi_damageable (Variables|Default|GetDamage) Hit%20Location))
      (bind _damageable (Default|GetDamageable _asi_damageable))
      (return _receiver_died _damageable))
    (:CastFailed
      (return false 0))))

(fn ReportHittoOwner
  (params (Instigator :type Actor%20Object%20Reference) (Enemy%20Died :type Boolean) (Damageable :type AC%20Damageable%20Object%20Reference))
  (bind _asplayer_character (Utilities|Casting|CastToPlayerCharacter Instigator))
  (Default|HitEnemy _asplayer_character Enemy%20Died Damageable))

(fn AddRecoil
  (Variables|Default|SetShoot_Recoil (Math|Float|Min(Float) (+ (Variables|Default|GetShoot_Recoil) (Variables|Default|GetShoot_RecoilIncrease)) (Variables|Default|GetShoot_RecoilMax))))

(fn UpdateRecoil
  (params (Delta%20Time :type Float%20%28single-precision%29))
  (Variables|Default|SetShoot_Recoil (Math|Float|Max(Float) (- (Variables|Default|GetShoot_Recoil) (* Delta%20Time (Variables|Default|GetShoot_RecoilRecover))) (Variables|Default|GetShoot_RecoilBase))))

(fn GetRecoil
  (bind _shoot_recoil (Variables|Default|GetShoot_Recoil))
  (bind _shoot_recoil_2 (Variables|Default|GetShoot_Recoil))
  (return (Math|Rotator|MakeRotator 0.0 (Math|Random|RandomFloatinRange (* _shoot_recoil -1.0) _shoot_recoil) (Math|Random|RandomFloatinRange (* _shoot_recoil_2 -1.0) _shoot_recoil_2))))