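; SMG weapon Blueprint that renders each shot as an electric arc and damages the hit actor.
; It implements Spawn Projectile with no moving projectile, spawning an Electric_World effect stretched from the start to the target location, which fades out and destroys itself.
; Damage applies immediately, and its death and damageable results feed a hit report to the owner.
; The construction script only calls the parent.
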(fn ConstructionScript
  (|CallParentFunction))

(fn SpawnProjectile
  (params (Instigator :type Base%20Character%20Object%20Reference) (FromLocation :type Vector :default "0, 0, 0") (ToLocation :type Vector :default "0, 0, 0") (HitNormal :type Vector :default "0, 0, 0") (HitActor :type Actor%20Object%20Reference) (Bounce%20Count :type Integer))
  (bind _returnvalue (Game|SpawnActorfromClass "/Game/Assets/Blueprints/Weapons/Projectiles/Electric_World.Electric_World_C" (Math|Transform|MakeTransform FromLocation (Transformation|GetWorldRotation (Variables|Character|GetMesh))) "Undefined" 0 0))
  (Default|SetEnd _returnvalue ToLocation)
  (Default|AutoSetSpikes _returnvalue 1.0)
  (Default|FadeOut _returnvalue 1.0 true)
  (bind (_enemy_died _damageable) (CallFunction|DealDamage HitActor ToLocation))
  (CallFunction|ReportHittoOwner Instigator _enemy_died _damageable))