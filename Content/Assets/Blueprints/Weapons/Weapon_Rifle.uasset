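; Rifle weapon that fires instant-hit electric shots which ricochet off surfaces.
; SpawnProjectile draws a fading Electric_World beam between two points, deals damage at the hit and reports the result to the instigator.
; It then calls Bounce, which checks the bounce count, waits a delay and re-enters SpawnProjectile.
; Each ricochet line-traces along the reflection of the previous segment to find the next endpoint and hit actor.
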(event Custom|Bounce
  (params (Instigator :type Base%20Character%20Object%20Reference) (From%20Location :type Vector) (To%20Location :type Vector) (Hit%20Normal :type Vector) (Hit%20Actor :type Actor%20Object%20Reference) (Bounce%20Count :type Integer))
  (if (<= Bounce%20Count (Variables|Default|GetBounce_Count))
    (Utilities|FlowControl|Delay (Variables|Default|GetBounce_Delay))
    (CallFunction|SpawnProjectile Instigator From%20Location To%20Location Hit%20Normal Hit%20Actor Bounce%20Count)))

(fn ConstructionScript
  (|CallParentFunction))

(fn SpawnProjectile
  (params (Instigator :type Base%20Character%20Object%20Reference) (FromLocation :type Vector :default "0, 0, 0") (ToLocation :type Vector :default "0, 0, 0") (HitNormal :type Vector :default "0, 0, 0") (HitActor :type Actor%20Object%20Reference) (Bounce%20Count :type Integer))
  (LocalVariables|SetM_Instigator Instigator)
  (LocalVariables|SetM_From FromLocation)
  (LocalVariables|SetM_To ToLocation)
  (LocalVariables|SetM_Normal HitNormal)
  (LocalVariables|SetM_HitActor HitActor)
  (bind _output_get (LocalVariables|SetM_BounceCount Bounce%20Count))
  (if (== _output_get 0)
    _
    (else
      (bind _outhit (Collision|LineTraceByChannel (+ (Math|Vector|Normalize (Math|Vector|GetReflectionVector (- (LocalVariables|GetM_To) (LocalVariables|GetM_From)) (LocalVariables|GetM_Normal))) (LocalVariables|GetM_To)) (+ (* (Math|Vector|Normalize (Math|Vector|GetReflectionVector (- (LocalVariables|GetM_To) (LocalVariables|GetM_From)) (LocalVariables|GetM_Normal))) 1e+04) (LocalVariables|GetM_To)) "TraceTypeQuery3" false 0 "None"))
      (LocalVariables|SetM_From (LocalVariables|GetM_To))
      (LocalVariables|SetM_To (select (.bBlockingHit (Collision|BreakHitResult _outhit)) (.Location (Collision|BreakHitResult _outhit)) (.TraceEnd (Collision|BreakHitResult _outhit))))
      (LocalVariables|SetM_Normal (.Normal (Collision|BreakHitResult _outhit)))
      (LocalVariables|SetM_HitActor (.HitActor (Collision|BreakHitResult _outhit)))))
  (bind _returnvalue (Game|SpawnActorfromClass "/Game/Assets/Blueprints/Weapons/Projectiles/Electric_World.Electric_World_C" (Math|Transform|MakeTransform (LocalVariables|GetM_From)) "Undefined" 0 0))
  (Default|SetEnd _returnvalue (LocalVariables|GetM_To))
  (Default|AutoSetSpikes _returnvalue 1e+01)
  (Default|FadeOut _returnvalue 2.0 true)
  (bind (_enemy_died _damageable) (CallFunction|DealDamage (LocalVariables|GetM_HitActor) (LocalVariables|GetM_To)))
  (Variables|Default|SetM_EnemyDied _enemy_died)
  (Variables|Default|SetM_Damageable _damageable)
  (CallFunction|ReportHittoOwner (LocalVariables|GetM_Instigator) _enemy_died _damageable)
  (LocalVariables|SetM_BounceCount (+ (LocalVariables|GetM_BounceCount) 1))
  (CallFunction|Bounce (LocalVariables|GetM_Instigator) (LocalVariables|GetM_From) (LocalVariables|GetM_To) (LocalVariables|GetM_Normal) (LocalVariables|GetM_HitActor) (LocalVariables|GetM_BounceCount)))