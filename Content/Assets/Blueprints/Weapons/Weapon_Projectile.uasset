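; Projectile weapon Blueprint that fires by spawning a physical projectile actor aimed at a target location.
; Spawn Projectile caches the shot parameters, then spawns the projectile at the origin with a look-at rotation toward the target.
; It hands the projectile the weapon as shooter, the instigating character, damage and bounce limit.
; The hit normal, hit actor and current bounce count are stored but not passed on.
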(fn ConstructionScript
  (|CallParentFunction))

(fn SpawnProjectile
  (params (Instigator :type Base%20Character%20Object%20Reference) (FromLocation :type Vector :default "0, 0, 0") (ToLocation :type Vector :default "0, 0, 0") (HitNormal :type Vector :default "0, 0, 0") (HitActor :type Actor%20Object%20Reference) (Bounce%20Count :type Integer))
  (LocalVariables|SetM_Instigator Instigator)
  (LocalVariables|SetM_From FromLocation)
  (LocalVariables|SetM_To ToLocation)
  (LocalVariables|SetM_Normal HitNormal)
  (LocalVariables|SetM_HitActor HitActor)
  (LocalVariables|SetM_BounceCount Bounce%20Count)
  (bind _returnvalue (Game|SpawnActorfromClass "/Game/Assets/Blueprints/Weapons/Projectiles/PhysicalProjectile.PhysicalProjectile_C" (Math|Transform|MakeTransform (LocalVariables|GetM_From) (Math|Rotator|FindLookatRotation (LocalVariables|GetM_From) (LocalVariables|GetM_To))) "Undefined" 0 (LocalVariables|GetM_Instigator)))
  (Variables|/Game/Assets/Blueprints/Weapons/Projectiles/PhysicalProjectile.PhysicalProjectile_C|SetShooter _returnvalue self)
  (Variables|/Game/Assets/Blueprints/Weapons/Projectiles/PhysicalProjectile.PhysicalProjectile_C|SetBaseCharacterInstigator _returnvalue (LocalVariables|GetM_Instigator))
  (Variables|/Game/Assets/Blueprints/Weapons/Projectiles/PhysicalProjectile.PhysicalProjectile_C|SetDamage _returnvalue (Variables|Default|GetDamage))
  (Variables|/Game/Assets/Blueprints/Weapons/Projectiles/PhysicalProjectile.PhysicalProjectile_C|SetMaxBounces _returnvalue (Variables|Default|GetMax%20Bounces)))