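; Shotgun weapon that fires a spread of hitscan pellets drawn as fading electric beams.
; SpawnProjectile calls itself once per pellet, line tracing along the aim direction offset in a circular pattern scaled by ShootRecoilBase.
; Each pellet spawns an Electric_World beam, deals damage to the hit actor and reports the result to the instigator.
; After the last pellet it resets the count and calls ShotgunBoost on the player character with the aim direction.
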(fn ConstructionScript
  (|CallParentFunction))

(fn SpawnProjectile
  (params (Instigator :type Base%20Character%20Object%20Reference) (FromLocation :type Vector :default "0, 0, 0") (ToLocation :type Vector :default "0, 0, 0") (HitNormal :type Vector :default "0, 0, 0") (HitActor :type Actor%20Object%20Reference) (Bounce%20Count :type Integer))
  (bind _shoot_recoilbase (Variables|Default|GetShoot_RecoilBase))
  (LocalVariables|SetM_Instigator Instigator)
  (LocalVariables|SetM_From FromLocation)
  (LocalVariables|SetM_To ToLocation)
  (LocalVariables|SetM_Normal HitNormal)
  (LocalVariables|SetM_HitActor HitActor)
  (LocalVariables|SetM_BounceCount Bounce%20Count)
  (if (< (Variables|Default|GetM_ShotgunPelletCount) (Variables|Default|GetShotgunPellets))
    (bind _outhit (Collision|LineTraceByChannel (LocalVariables|GetM_From) (+ (LocalVariables|GetM_From) (* (Math|Vector|RotateVector (Math|Vector|Normalize (- (LocalVariables|GetM_To) (LocalVariables|GetM_From))) (Math|Rotator|MakeRotator (* (Math|Trig|Sin(Degrees) (* (Variables|Default|GetM_ShotgunPelletCount) (/ 3.6e+02 (Math|Conversions|ToFloat(Integer) (Variables|Default|GetShotgunPellets))))) _shoot_recoilbase) (* (Math|Trig|Sin(Degrees) (* (Variables|Default|GetM_ShotgunPelletCount) (/ 3.6e+02 (Math|Conversions|ToFloat(Integer) (Variables|Default|GetShotgunPellets))))) _shoot_recoilbase) (* (Math|Trig|Cos(Degrees) (* (Variables|Default|GetM_ShotgunPelletCount) (/ 3.6e+02 (Math|Conversions|ToFloat(Integer) (Variables|Default|GetShotgunPellets))))) _shoot_recoilbase))) 3e+03)) "TraceTypeQuery3" false 0 "None"))
    (LocalVariables|SetM_ToPellet (select (.bBlockingHit (Collision|BreakHitResult _outhit)) (.Location (Collision|BreakHitResult _outhit)) (+ (LocalVariables|GetM_From) (* (Math|Vector|RotateVector (Math|Vector|Normalize (- (LocalVariables|GetM_To) (LocalVariables|GetM_From))) (Math|Rotator|MakeRotator (* (Math|Trig|Sin(Degrees) (* (Variables|Default|GetM_ShotgunPelletCount) (/ 3.6e+02 (Math|Conversions|ToFloat(Integer) (Variables|Default|GetShotgunPellets))))) _shoot_recoilbase) (* (Math|Trig|Sin(Degrees) (* (Variables|Default|GetM_ShotgunPelletCount) (/ 3.6e+02 (Math|Conversions|ToFloat(Integer) (Variables|Default|GetShotgunPellets))))) _shoot_recoilbase) (* (Math|Trig|Cos(Degrees) (* (Variables|Default|GetM_ShotgunPelletCount) (/ 3.6e+02 (Math|Conversions|ToFloat(Integer) (Variables|Default|GetShotgunPellets))))) _shoot_recoilbase))) 3e+03))))
    (Variables|Default|SetM_ShotgunPelletCount (+ (Variables|Default|GetM_ShotgunPelletCount) 1))
    (LocalVariables|SetM_HitActor (.HitActor (Collision|BreakHitResult _outhit)))
    (bind _returnvalue (Game|SpawnActorfromClass "/Game/Assets/Blueprints/Weapons/Projectiles/Electric_World.Electric_World_C" (Math|Transform|MakeTransform (LocalVariables|GetM_From)) "Undefined" 0 0))
    (Default|SetEnd _returnvalue (LocalVariables|GetM_ToPellet))
    (Default|AutoSetSpikes _returnvalue 5e+01)
    (Default|FadeOut _returnvalue 1.0 true)
    (bind (_enemy_died _damageable) (CallFunction|DealDamage (LocalVariables|GetM_HitActor) (LocalVariables|GetM_ToPellet)))
    (CallFunction|ReportHittoOwner (LocalVariables|GetM_Instigator) _enemy_died _damageable)
    (LocalVariables|SetM_BounceCount (+ (LocalVariables|GetM_BounceCount) 1))
    (CallFunction|SpawnProjectile (LocalVariables|GetM_Instigator) (LocalVariables|GetM_From) (LocalVariables|GetM_To) (LocalVariables|GetM_Normal) (LocalVariables|GetM_HitActor) (LocalVariables|GetM_BounceCount))
    (else
      (Variables|Default|SetM_ShotgunPelletCount 0)
      (bind _asplayer_character (Utilities|Casting|CastToPlayerCharacter (LocalVariables|GetM_Instigator)))
      (Default|ShotgunBoost _asplayer_character (Math|Vector|Normalize (- (LocalVariables|GetM_To) (LocalVariables|GetM_From)))))))