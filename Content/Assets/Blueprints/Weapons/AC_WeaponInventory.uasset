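; Weapon inventory component that holds one slot each for rifle, SMG, shotgun, sniper and projectile weapons, and handles pickup, switching and firing.
; AddWeapon casts a pickup to its type, stores it hidden, then equips it if nothing is held or auto-switch is on.
; Duplicates, and any projectile weapon picked up by a PlayerCharacter, are destroyed to add ammo to all owned weapons.
; SwitchTo swaps mesh visibility, and shooting is forwarded to the current weapon.
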(event EventBeginPlay)

(event EventTick
  (params (DeltaSeconds :type Float%20%28single-precision%29)))

(fn AddWeapon
  (params (Weapon :type Weapon%20Object%20Reference) (Holder :type Base%20Character%20Object%20Reference))
  (LocalVariables|Setm_Weapon Weapon)
  (LocalVariables|Setm_Holder Holder)
  (bind _can_pick_up (Default|CanPickUp (LocalVariables|Getm_Weapon)))
  (if _can_pick_up
    (bind _asweapon_rifle (Utilities|Casting|CastToWeapon_Rifle (LocalVariables|Getm_Weapon))
      (:then
        (if (!= (Variables|Default|GetRifle) 0)
          _
          (else
            (Variables|Default|SetRifle _asweapon_rifle)
            (Default|PickUp (LocalVariables|Getm_Weapon) (LocalVariables|Getm_Holder) :!label _label)
            (Rendering|SetVisibility (Variables|/Game/Assets/Blueprints/Weapons/Weapon.Weapon_C|GetMesh (LocalVariables|Getm_Weapon)) false true)
            (if (== (Variables|Default|GetCurrent%20Weapon) 0)
              (CallFunction|Switchto (LocalVariables|Getm_Weapon) :!label _label_2)
              (elif (Variables|Default|GetAuto%20Switch%20To%20New%20Weapon)
                (goto _label_2)
                (else
                  _)))
            (return true))))
      (:CastFailed
        (bind _asweapon_smg (Utilities|Casting|CastToWeapon_SMG (LocalVariables|Getm_Weapon))
          (:then
            (if (!= (Variables|Default|GetSMG) 0)
              _
              (else
                (Variables|Default|SetSMG _asweapon_smg)
                (goto _label))))
          (:CastFailed
            (bind _asweapon_shotgun (Utilities|Casting|CastToWeapon_Shotgun (LocalVariables|Getm_Weapon))
              (:then
                (if (!= (Variables|Default|GetShotgun) 0)
                  _
                  (else
                    (Variables|Default|SetShotgun _asweapon_shotgun)
                    (goto _label))))
              (:CastFailed
                (bind _asweapon_sniper (Utilities|Casting|CastToWeapon_Sniper (LocalVariables|Getm_Weapon))
                  (:then
                    (if (!= (Variables|Default|GetSniper) 0)
                      _
                      (else
                        (Variables|Default|SetSniper _asweapon_sniper)
                        (goto _label))))
                  (:CastFailed
                    (bind _asweapon_projectile (Utilities|Casting|CastToWeapon_Projectile (LocalVariables|Getm_Weapon))
                      (:then
                        (Utilities|Casting|CastToPlayerCharacter (LocalVariables|Getm_Holder)
                          (:then
                            _)
                          (:CastFailed
                            (if (!= (Variables|Default|GetProjectile) 0)
                              _
                              (else
                                (Variables|Default|SetProjectile _asweapon_projectile)
                                (goto _label))))))
                      (:CastFailed
                        (return false)))))))))))
    (CallFunction|AddAmmotoAllWeapons)
    (Actor|DestroyActor (LocalVariables|Getm_Weapon))
    (Audio|PlaySoundatLocation "/Game/3rdParty/Audio/Sounds/weapon_switch.weapon_switch" (Transformation|GetActorLocation (LocalVariables|Getm_Holder)) "0, 0, 0" 1.0 1.0 0.0 0 0 0)
    (return false)
    (else
      (return false))))

(fn HasCurrentWeapon
  (return (!= (Variables|Default|GetCurrent%20Weapon) 0)))

(fn TryShootCurrentWeapon
  (params (Instigator :type Base%20Character%20Object%20Reference))
  (bind _has_current_weapon (CallFunction|HasCurrentWeapon))
  (if _has_current_weapon
    (bind _shot (Default|Shoot (Variables|Default|GetCurrent%20Weapon) Instigator))
    (return _shot)))

(fn Switchto
  (params (Weapon :type Weapon%20Object%20Reference))
  (if (not (== Weapon 0))
    (bind _has_current_weapon (CallFunction|HasCurrentWeapon))
    (if _has_current_weapon
      (Rendering|SetVisibility (Variables|/Game/Assets/Blueprints/Weapons/Weapon.Weapon_C|GetMesh (Variables|Default|GetCurrent%20Weapon)) false true))
    (bind _output_get (Variables|Default|SetCurrent%20Weapon Weapon))
    (Rendering|SetVisibility (Variables|/Game/Assets/Blueprints/Weapons/Weapon.Weapon_C|GetMesh _output_get) true true)))

(fn AddAmmotoAllWeapons
  (bind _sniper (Variables|Default|GetSniper))
  (bind _projectile (Variables|Default|GetProjectile))
  (bind _shotgun (Variables|Default|GetShotgun))
  (bind _rifle (Variables|Default|GetRifle))
  (bind _smg (Variables|Default|GetSMG))
  (if (!= _rifle 0)
    (Default|AddAmmo _rifle 6))
  (if (!= _smg 0)
    (Default|AddAmmo _smg 24))
  (if (!= _shotgun 0)
    (Default|AddAmmo _shotgun 2))
  (if (!= _sniper 0)
    (Default|AddAmmo _sniper 1))
  (if (!= _projectile 0)
    (Default|AddAmmo _projectile 2)))

(fn RemoveCurrentWeapon
  (Variables|Default|SetCurrent%20Weapon 0))