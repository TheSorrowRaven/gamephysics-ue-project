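; Weapon spawner actor that keeps a pickup of its configured Weapon class available at its location.
; BeginPlay spawns the weapon at the spawner's transform and stores it in SpawnedWeapon.
; Tick feeds a Cooldown Delay back into the same check, spawning a replacement whenever the stored weapon is invalid or can no longer be picked up.
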(event EventBeginPlay
  (if (not (Utilities|IsValid (Variables|Default|GetSpawned%20Weapon)))
    (bind _returnvalue (Game|SpawnActorfromClass (Variables|Default|GetWeapon) (Transformation|GetActorTransform) "AdjustIfPossibleButAlwaysSpawn" 0 0 :!label _label))
    (Variables|Default|SetSpawned%20Weapon _returnvalue)
    (else
      (bind _can_pick_up (Default|CanPickUp (Variables|Default|GetSpawned%20Weapon)))
      (if (not _can_pick_up)
        (goto _label)))))

(event Collision|EventActorBeginOverlap
  (params (OtherActor :type Actor%20Object%20Reference)))

(event EventTick
  (params (DeltaSeconds :type Float%20%28single-precision%29))
  (Utilities|FlowControl|Delay (Variables|Default|GetCooldown))
  (if (not (Utilities|IsValid (Variables|Default|GetSpawned%20Weapon)))
    (bind _returnvalue (Game|SpawnActorfromClass (Variables|Default|GetWeapon) (Transformation|GetActorTransform) "AdjustIfPossibleButAlwaysSpawn" 0 0 :!label _label))
    (Variables|Default|SetSpawned%20Weapon _returnvalue)
    (else
      (bind _can_pick_up (Default|CanPickUp (Variables|Default|GetSpawned%20Weapon)))
      (if (not _can_pick_up)
        (goto _label)))))

(fn ConstructionScript)