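; FinishTutorial is a level component that ends the tutorial once every enemy in its Enemies array has died.
; A Tick throttled by a short Delay recounts deaths through each enemy's ACDamageable and shows the remaining count on a text render.
; At zero, a Loaded flag guards a one-time finish that enables the player HUD's next-level text, waits, then loads Level_1 as a level instance and unloads Level_Tutorial.
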(event EventTick
  (params (DeltaSeconds :type Float%20%28single-precision%29))
  (Utilities|FlowControl|Delay 0.1)
  (Variables|Default|SetDead%20Enemies 0)
  (for _array_element (Variables|Default|GetEnemies)
    (if (Variables|/Game/Assets/Blueprints/Characters/AC_Damageable.AC_Damageable_C|GetHasDied (Variables|/Game/Assets/Blueprints/Characters/BaseCharacter.BaseCharacter_C|GetAC_Damageable _array_element))
      (Math|Integer|IncrementInt (Variables|Default|GetDead%20Enemies))))
  (Rendering|Components|TextRender|SetText (Variables|Default|GetTextRender1) (Utilities|Text|ToText(Integer) (- (Utilities|Array|Length (Variables|Default|GetEnemies)) (Variables|Default|GetDead%20Enemies))))
  (if (== (Variables|Default|GetDead%20Enemies) (Utilities|Array|Length (Variables|Default|GetEnemies)))
    (if (not (Variables|Default|GetLoaded))
      (Variables|Default|SetLoaded true)
      (Development|PrintString "Finish")
      (bind _asplayer_character (Utilities|Casting|CastToPlayerCharacter (Game|GetPlayerCharacter 0)))
      (Default|EnableNextLevelText (Variables|/Game/Assets/Blueprints/Characters/PlayerCharacter.PlayerCharacter_C|GetHUD _asplayer_character))
      (Utilities|FlowControl|Delay 4.0)
      (Class|LevelStreamingDynamic|LoadLevelInstancebySoftObjectPtr "/Game/Assets/Maps/Level_1.Level_1" "0, 0, 0" "0, 0, 0")
      (Class|GameplayStatics|UnloadStreamLevelbySoftObjectPtr "/Game/Assets/Maps/Level_Tutorial.Level_Tutorial" false))))

(fn ConstructionScript)