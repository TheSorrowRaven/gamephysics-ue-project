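; Objective actor that the level attaches to a parent component, counting toward the player's objective number.
; Its AttachToParent event disables physics and collision, snaps it to the given parent and moves its mesh to lighting channel 1.
; It then sets the player character's EnergyRecover to a high value, increments ObjectiveNumber and updates the end vector on six Niagara effects.
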(event Custom|Attach%20To%20Parent
  (params (Parent :type Scene%20Component%20Object%20Reference))
  (bind _box (Variables|Default|GetBox))
  (bind _scale (Variables|Default|GetScale))
  (Physics|SetSimulatePhysics _box false)
  (Collision|SetCollisionEnabled _box "NoCollision")
  (Collision|SetCollisionEnabled (Variables|Default|GetSphere) "NoCollision")
  (Transformation|AttachComponentToComponent Parent "None" "SnapToTarget" "SnapToTarget" "SnapToTarget" true)
  (Rendering|Components|SetLightingChannels (Variables|Default|GetStaticMesh) false true false)
  (bind _asplayer_character (Utilities|Casting|CastToPlayerCharacter (Game|GetPlayerCharacter 0)))
  (Variables|/Game/Assets/Blueprints/Characters/PlayerCharacter.PlayerCharacter_C|SetEnergy_Recover _asplayer_character 1e+03)
  (Math|Integer|IncrementInt (Variables|/Game/Assets/Blueprints/Characters/PlayerCharacter.PlayerCharacter_C|GetObjectiveNumber _asplayer_character)
    (:%20%20
      (Niagara|SetNiagaraVariable(Vector3) (Variables|Default|GetNiagara) "User.End" _scale)
      (Niagara|SetNiagaraVariable(Vector3) (Variables|Default|GetNiagara1) "User.End" _scale)
      (Niagara|SetNiagaraVariable(Vector3) (Variables|Default|GetNiagara2) "User.End" _scale)
      (Niagara|SetNiagaraVariable(Vector3) (Variables|Default|GetNiagara3) "User.End" _scale)
      (Niagara|SetNiagaraVariable(Vector3) (Variables|Default|GetNiagara4) "User.End" _scale)
      (Niagara|SetNiagaraVariable(Vector3) (Variables|Default|GetNiagara5) "User.End" _scale)
      (Development|PrintString "SETT"))))

(event EventBeginPlay)

(event Collision|EventActorBeginOverlap
  (params (OtherActor :type Actor%20Object%20Reference)))

(event EventTick
  (params (DeltaSeconds :type Float%20%28single-precision%29)))

(fn ConstructionScript)