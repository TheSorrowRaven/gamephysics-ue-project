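; StartLevel is a level component that places the player at a start point when a level begins.
; After a zero-length delay on BeginPlay, it moves the PlayerCharacter to the Start actor's location and rotation.
; It then disables the HUD's next-level text, if a HUD exists, and calls StartObjective on the character.
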(event EventBeginPlay
  (bind _returnvalue (Game|GetPlayerCharacter 0))
  (bind _start (Variables|Default|GetStart))
  (Utilities|FlowControl|Delay 0.0)
  (if (Utilities|IsValid _returnvalue)
    (bind _asplayer_character (Utilities|Casting|CastToPlayerCharacter _returnvalue))
    (Utilities|FlowControl|Sequence
      (:then_0
        (Transformation|SetActorLocationAndRotation _asplayer_character (Transformation|GetActorLocation _start) (Transformation|GetActorRotation _start))
        (bind _asplayer_character_2 (Utilities|Casting|CastToPlayerCharacter (Game|GetPlayerCharacter 0)))
        (if (!= (Variables|/Game/Assets/Blueprints/Characters/PlayerCharacter.PlayerCharacter_C|GetHUD _asplayer_character_2) 0)
          (Default|DisableNextLevelText (Variables|/Game/Assets/Blueprints/Characters/PlayerCharacter.PlayerCharacter_C|GetHUD _asplayer_character_2))))
      (:then_1
        (Default|StartObjective _asplayer_character)))))

(fn ConstructionScript)