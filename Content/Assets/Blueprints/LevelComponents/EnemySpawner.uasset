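; EnemySpawner is a level actor that repeatedly spawns Enemy_SFC enemies at random ground points within its footprint, once StartSpawningEnemies switches it on.
; While active, Tick runs through a Delay of SpawnRate, which paces spawns.
; Each cycle picks random XY offsets from the static mesh's scaled bounds and line-traces downward from above on the Visibility channel.
; A blocking hit spawns an enemy slightly above it, adjusting for collisions.
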(event Custom|Start%20Spawning%20Enemies
  (Variables|Default|SetStartSpawning true))

(event EventBeginPlay)

(event Collision|EventActorBeginOverlap
  (params (OtherActor :type Actor%20Object%20Reference)))

(event EventTick
  (params (DeltaSeconds :type Float%20%28single-precision%29))
  (bind _returnvalue (Transformation|GetActorScale3D))
  (bind _returnvalue_2 (Transformation|GetActorScale3D))
  (bind _returnvalue_3 (Transformation|GetActorLocation))
  (bind _staticmesh (Variables|Default|GetStaticMesh))
  (bind (_min _max) (Components|StaticMesh|GetLocalBounds _staticmesh))
  (bind _returnvalue_4 (* (.x _max) (.x _returnvalue_2)))
  (bind _returnvalue_5 (* (.x _min) (.x _returnvalue_2)))
  (bind _returnvalue_6 (* (.y _min) (.y _returnvalue)))
  (bind _returnvalue_7 (* (.y _max) (.y _returnvalue)))
  (bind _returnvalue_8 (Math|Random|RandomFloatinRange _returnvalue_6 _returnvalue_7))
  (bind _returnvalue_9 (Math|Random|RandomFloatinRange _returnvalue_5 _returnvalue_4))
  (bind _returnvalue_10 (Math|Vector|MakeVector _returnvalue_9 _returnvalue_8 1e+03))
  (bind _returnvalue_11 (+ _returnvalue_3 _returnvalue_10))
  (if (Variables|Default|GetStartSpawning)
    (Utilities|FlowControl|Delay (Variables|Default|GetSpawn%20Rate))
    (bind _outhit (Collision|LineTraceByChannel _returnvalue_11 (+ _returnvalue_11 (* (Math|Vector|VectorDown) 1e+04)) "TraceTypeQuery1" false 0 "None"))
    (if (.bBlockingHit (Collision|BreakHitResult _outhit))
      (Game|SpawnActorfromClass "/Game/Assets/Blueprints/Characters/Enemy_SFC.Enemy_SFC_C" (Math|Transform|MakeTransform (+ (.Location (Collision|BreakHitResult _outhit)) "0, 0,96.000000")) "AdjustIfPossibleButAlwaysSpawn" 0 0))))

(fn ConstructionScript)