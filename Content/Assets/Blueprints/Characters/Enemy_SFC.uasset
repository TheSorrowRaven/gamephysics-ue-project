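; Enemy character that spawns with a projectile weapon, aims at the player and shoots, with no movement logic of its own.
; Each tick, while both are alive, the game is unfinished and the player is in range, it turns yaw, head and gun toward them.
; It fires when a head-to-player trace is clear, topping up ammo after each attempt.
; Damage and death hooks play sounds; death also ragdolls it and drops the weapon.
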(event EventBeginPlay
  (bind _returnvalue (Game|SpawnActorfromClass "/Game/Assets/Blueprints/Weapons/Weapon_Projectile.Weapon_Projectile_C" (Math|Transform|MakeTransform "0, 0, 0") "Undefined" 0 0))
  (CallFunction|PickupWeapon _returnvalue)
  (Default|AddAmmo _returnvalue 4))

(event EventTick
  (params (DeltaSeconds :type Float%20%28single-precision%29))
  (bind _returnvalue (Transformation|GetActorLocation))
  (bind _gun_look (Variables|Default|GetGun%20Look))
  (if (not (Variables|/Game/Assets/Blueprints/Characters/AC_Damageable.AC_Damageable_C|GetHasDied (Variables|Default|GetAC_Damageable)))
    ;[1 1 1] Rotation
    (bind _asplayer_character (Utilities|Casting|CastToPlayerCharacter (Game|Player|GetPlayerPawn 0)))
    (if (not (Variables|/Game/Assets/Blueprints/Characters/AC_Damageable.AC_Damageable_C|GetHasDied (Variables|/Game/Assets/Blueprints/Characters/BaseCharacter.BaseCharacter_C|GetAC_Damageable _asplayer_character)))
      (if (not (Variables|/Game/Assets/Blueprints/Characters/PlayerCharacter.PlayerCharacter_C|GetFinished%20Game _asplayer_character))
        (if (< (Math|Vector|VectorLength (- _returnvalue (Transformation|GetWorldLocation (Variables|/Game/Assets/Blueprints/Characters/BaseCharacter.BaseCharacter_C|GetCharacter%20Look _asplayer_character)))) 4e+03)
          (Transformation|SetActorRotation (Math|Rotator|MakeRotator 0.0 0.0 (.yaw (Math|Rotator|FindLookatRotation _returnvalue (Transformation|GetWorldLocation (Variables|/Game/Assets/Blueprints/Characters/BaseCharacter.BaseCharacter_C|GetCharacter%20Look _asplayer_character))))))
          (CallFunction|UpdateHeadRotation false)
          (Transformation|SetWorldRotation _gun_look (Math|Rotator|FindLookatRotation (Transformation|GetWorldLocation _gun_look) (Transformation|GetWorldLocation (Variables|/Game/Assets/Blueprints/Characters/BaseCharacter.BaseCharacter_C|GetCharacter%20Look _asplayer_character))) false false)
          ;[1 1 1] Shoot
          (bind _asplayer_character_2 (Utilities|Casting|CastToPlayerCharacter (Game|Player|GetPlayerPawn 0)))
          (bind _outhit (Collision|LineTraceByChannel (Transformation|GetSocketLocation (Variables|Character|GetMesh) "head") (Transformation|GetWorldLocation (Variables|/Game/Assets/Blueprints/Characters/BaseCharacter.BaseCharacter_C|GetCharacter%20Center _asplayer_character_2)) "TraceTypeQuery3" false 0 "None"))
          (if (not (and (.bBlockingHit (Collision|BreakHitResult _outhit)) (not (== _asplayer_character_2 (.HitActor (Collision|BreakHitResult _outhit))))))
            (CallFunction|TryShootCurrentWeapon)
            (Default|AddAmmo (Variables|/Game/Assets/Blueprints/Weapons/AC_WeaponInventory.AC_WeaponInventory_C|GetCurrent%20Weapon (Variables|Default|GetAC_WeaponInventory)) 1)))))))

(fn ConstructionScript
  (Variables|Default|SetAttach%20Gun%20To%20Component (Variables|Default|GetGun%20Look)))

(fn ChildDie
  (bind _ac_weaponinventory (Variables|Default|GetAC_WeaponInventory))
  (Pawn|Components|CharacterMovement|DisableMovement (Variables|Character|GetCharacterMovement))
  (Variables|/Script/Engine.PrimitiveComponent|SetbIgnoreRadialImpulse (Variables|Default|GetCapsuleComponent) false)
  (Audio|SpawnSoundatLocation "/Game/3rdParty/Audio/Sounds/enemy_die.enemy_die" (Transformation|GetActorLocation) "0, 0, 0" 1.0 1.0 0.0 0 0)
  (CallFunction|Ragdoll)
  (Physics|AddRadialImpulse (Variables|Character|GetMesh) (Variables|Default|GetHit%20Location) 1e+02 1e+03 "RIF_Constant" true)
  (bind _has_current_weapon (Default|HasCurrentWeapon _ac_weaponinventory))
  (if _has_current_weapon
    (Default|DropWeapon (Variables|/Game/Assets/Blueprints/Weapons/AC_WeaponInventory.AC_WeaponInventory_C|GetCurrent%20Weapon _ac_weaponinventory))
    (Default|RemoveCurrentWeapon _ac_weaponinventory)))

(fn Ragdoll
  (Collision|SetCollisionEnabled (Variables|Default|GetCapsuleComponent) "NoCollision")
  (Physics|SetSimulatePhysics (Variables|Character|GetMesh) true)
  (Class|PrimitiveComponent|AddForceatLocation (Variables|Character|GetMesh) "0.000000, 0,100000.000000" (Variables|Default|GetHit%20Location) "None"))

(fn ChildReceiveDamage
  (Audio|PlaySoundatLocation "/Game/3rdParty/Audio/Sounds/enemy_hit.enemy_hit" (Transformation|GetActorLocation) "0, 0, 0" 1.0 1.0 0.0 0 0 0))