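; Boss enemy character Blueprint that extends a parent enemy class with a pair of firing arm guns.
; Tick counts down a fire-rate cooldown and, while CanShoot is true, fires the left gun, then the right gun after half the interval for alternating shots.
; Both guns call Shoot2 with shared size, damage and material settings, while BeginPlay primes the cooldown and calls the parent.
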(event EventBeginPlay
  (|CallParentFunction)
  (Variables|Default|SetArm%20Guns%20Fire%20Rate%20Cooldown (Variables|Default|GetArm%20Guns%20Fire%20Rate)))

(event Collision|EventActorBeginOverlap
  (params (OtherActor :type Actor%20Object%20Reference))
  (|CallParentFunction OtherActor) ; This node is disabled and will not be called.\nDrag off pins to build functionality.
)

(event EventTick
  (params (DeltaSeconds :type Float%20%28single-precision%29))
  (|CallParentFunction DeltaSeconds)
  (Utilities|FlowControl|Sequence
    (:then_0
      (Variables|Default|SetArm%20Guns%20Fire%20Rate%20Cooldown (- (Variables|Default|GetArm%20Guns%20Fire%20Rate%20Cooldown) DeltaSeconds)))
    (:then_1
      (if (Variables|Default|GetCan%20Shoot)
        (if (< (Variables|Default|GetArm%20Guns%20Fire%20Rate%20Cooldown) 0.0)
          (Variables|Default|SetArm%20Guns%20Fire%20Rate%20Cooldown (Variables|Default|GetArm%20Guns%20Fire%20Rate))
          (CallFunction|Shoot2 (Variables|Default|GetProjectile%20Spawn_Left) (Variables|Default|GetArm%20Guns%20Projectile%20Size) (Variables|Default|GetArm%20Guns%20Damage) (Variables|Default|GetArm%20Guns%20Material))
          (Utilities|FlowControl|Delay (/ (Variables|Default|GetArm%20Guns%20Fire%20Rate) 2.0))
          (CallFunction|Shoot2 (Variables|Default|GetProjectile%20Spawn_Right) (Variables|Default|GetArm%20Guns%20Projectile%20Size) (Variables|Default|GetArm%20Guns%20Damage) (Variables|Default|GetArm%20Guns%20Material)))))))

(fn ConstructionScript
  (|CallParentFunction))