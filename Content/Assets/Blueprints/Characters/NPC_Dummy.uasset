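; NPC dummy character that watches the player and reacts to damage and death.
; While alive and within range of the player's CharacterLook, Tick optionally yaws the body toward it (TurnBody) and calls UpdateHeadRotation with the inverse flag.
; Child damage hook plays a hit sound.
; Child death hook disables movement, plays a death sound and ragdolls the mesh, launching it with upward force and a radial impulse at HitLocation.
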(event EventTick
  (params (DeltaSeconds :type Float%20%28single-precision%29))
  (bind _returnvalue (Transformation|GetActorLocation))
  (bind _turn_body (Variables|Default|GetTurn%20Body))
  (if (not (Variables|/Game/Assets/Blueprints/Characters/AC_Damageable.AC_Damageable_C|GetHasDied (Variables|Default|GetAC_Damageable)))
    ;[1 1 1] Rotation
    (bind _asplayer_character (Utilities|Casting|CastToPlayerCharacter (Game|Player|GetPlayerPawn 0)))
    (if (< (Math|Vector|VectorLength (- _returnvalue (Transformation|GetWorldLocation (Variables|/Game/Assets/Blueprints/Characters/BaseCharacter.BaseCharacter_C|GetCharacter%20Look _asplayer_character)))) 1e+04)
      (if _turn_body
        (Transformation|SetActorRotation (Math|Rotator|MakeRotator 0.0 0.0 (.yaw (Math|Rotator|FindLookatRotation _returnvalue (Transformation|GetWorldLocation (Variables|/Game/Assets/Blueprints/Characters/BaseCharacter.BaseCharacter_C|GetCharacter%20Look _asplayer_character)))))))
      (CallFunction|UpdateHeadRotation (not _turn_body)))))

(fn ConstructionScript
  (|CallParentFunction))

(fn Ragdoll
  (Collision|SetCollisionEnabled (Variables|Default|GetCapsuleComponent) "NoCollision")
  (Physics|SetSimulatePhysics (Variables|Character|GetMesh) true)
  (Class|PrimitiveComponent|AddForceatLocation (Variables|Character|GetMesh) "0.000000, 0,100000.000000" (Variables|Default|GetHit%20Location) "None"))

(fn ChildDie
  (Pawn|Components|CharacterMovement|DisableMovement (Variables|Character|GetCharacterMovement))
  (Variables|/Script/Engine.PrimitiveComponent|SetbIgnoreRadialImpulse (Variables|Default|GetCapsuleComponent) false)
  (Audio|SpawnSoundatLocation "/Game/3rdParty/Audio/Sounds/enemy_die.enemy_die" (Transformation|GetActorLocation) "0, 0, 0" 1.0 1.0 0.0 0 0)
  (CallFunction|Ragdoll)
  (Physics|AddRadialImpulse (Variables|Character|GetMesh) (Variables|Default|GetHit%20Location) 1e+02 1e+03 "RIF_Constant" true))

(fn ChildReceiveDamage
  (Audio|PlaySoundatLocation "/Game/3rdParty/Audio/Sounds/enemy_hit.enemy_hit" (Transformation|GetActorLocation) "0, 0, 0" 1.0 1.0 0.0 0 0 0))