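; Base character Blueprint that gives its child characters shared weapon handling, health and death behavior.
; An ACWeaponInventory component handles pickup, shooting and switching between four weapon types, while ACDamageable processes HP, damage and death through the damageable interface.
; Empty hook functions let children react to pickups, healing, damage and death.
; A helper aims head rotation at the player through either the enemy or SFC animation Blueprint.
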(event Custom|Pickup%20Weapon
  (params (Weapon :type Weapon%20Object%20Reference))
  ;[1 1 1] Weapon
  (bind _picked_up_weapon (Default|AddWeapon (Variables|Components|GetAC_WeaponInventory) Weapon self))
  (if _picked_up_weapon
    (Transformation|AttachComponentToComponent Weapon (Variables|Default|GetAttach%20Gun%20To%20Component) "None" "SnapToTarget" "SnapToTarget" "SnapToTarget" true)
    (CallFunction|WeaponPickedUp Weapon)))

(event EventHP
  (params (HP :type Float%20%28single-precision%29))
  ;[1 1 1] I_Damageable
  (Default|ReceiveHP (Variables|Components|GetAC_Damageable) HP)
  (CallFunction|ChildReceiveHP))

(event EventDie
  ;[1 1 1] I_Damageable
  (Default|Die (Variables|Components|GetAC_Damageable))
  (CallFunction|ChildDie))

(fn ConstructionScript)

(fn Shoot
  (Default|TryShootCurrentWeapon (Variables|Components|GetAC_WeaponInventory) self))

(fn TryShootCurrentWeapon
  (Default|TryShootCurrentWeapon (Variables|Components|GetAC_WeaponInventory) self))

(fn WeaponPickedUp
  (params (Weapon :type Weapon%20Object%20Reference)))

(fn SwitchtoRifle
  (bind _ac_weaponinventory (Variables|Components|GetAC_WeaponInventory))
  (Default|Switchto _ac_weaponinventory (Variables|/Game/Assets/Blueprints/Weapons/AC_WeaponInventory.AC_WeaponInventory_C|GetRifle _ac_weaponinventory)))

(fn SwitchtoSMG
  (bind _ac_weaponinventory (Variables|Components|GetAC_WeaponInventory))
  (Default|Switchto _ac_weaponinventory (Variables|/Game/Assets/Blueprints/Weapons/AC_WeaponInventory.AC_WeaponInventory_C|GetSMG _ac_weaponinventory)))

(fn SwitchtoShotgun
  (bind _ac_weaponinventory (Variables|Components|GetAC_WeaponInventory))
  (Default|Switchto _ac_weaponinventory (Variables|/Game/Assets/Blueprints/Weapons/AC_WeaponInventory.AC_WeaponInventory_C|GetShotgun _ac_weaponinventory)))

(fn SwitchtoSniper
  (bind _ac_weaponinventory (Variables|Components|GetAC_WeaponInventory))
  (Default|Switchto _ac_weaponinventory (Variables|/Game/Assets/Blueprints/Weapons/AC_WeaponInventory.AC_WeaponInventory_C|GetSniper _ac_weaponinventory)))

(fn ChildReceiveDamage)

(fn ChildReceiveHP)

(fn ChildDie)

(fn UpdateHeadRotation
  (params (Look%20Horizontal :type Boolean))
  (bind _mesh (Variables|Character|GetMesh))
  (bind _returnvalue (Components|SkeletalMesh|GetAnimInstance _mesh))
  (bind _asplayer_character (Utilities|Casting|CastToPlayerCharacter (Game|Player|GetPlayerPawn 0)))
  (bind _asenemy_anim_bp (Utilities|Casting|CastToEnemy_AnimBP _returnvalue)
    (:then
      (Variables|/Game/Mannequin/Character/Mesh/Enemy_AnimBP.Enemy_AnimBP_C|SetHeadRotation _asenemy_anim_bp (Math|Rotator|MakeRotator (* (.pitch (Math|Rotator|FindLookatRotation (Transformation|GetWorldLocation (Variables|Default|GetCharacter%20Look)) (Transformation|GetWorldLocation (Variables|BaseCharacter_C|GetCharacter%20Look _asplayer_character)))) -1.0) 0.0 (Math|Float|SelectFloat (.yaw (Math|Rotator|FindLookatRotation (Transformation|GetWorldLocation (Variables|Default|GetCharacter%20Look)) (Transformation|GetWorldLocation (Variables|BaseCharacter_C|GetCharacter%20Look _asplayer_character)))) 0.0 Look%20Horizontal))))
    (:CastFailed
      (bind _assfc_anim_blueprint (Utilities|Casting|CastToSFC_AnimBlueprint _returnvalue))
      (Variables|/Game/3rdParty/Characters/SciFiFPSCharacter/SFC_AnimBlueprint.SFC_AnimBlueprint_C|SetHeadRotation _assfc_anim_blueprint (Math|Rotator|MakeRotator (* (.pitch (Math|Rotator|FindLookatRotation (Transformation|GetWorldLocation (Variables|Default|GetCharacter%20Look)) (Transformation|GetWorldLocation (Variables|BaseCharacter_C|GetCharacter%20Look _asplayer_character)))) -1.0) 0.0 0.0)))))

(fn GetDamageable
  (return (Variables|Components|GetAC_Damageable)))

(fn ReceiveDamage
  (params (Damage :type Float%20%28single-precision%29) (Hit%20Location :type Vector :default "0, 0, 0"))
  (Variables|Default|SetHit%20Location Hit%20Location)
  (bind _died (Default|ReceiveDamage (Variables|Components|GetAC_Damageable) Damage Hit%20Location))
  (CallFunction|ChildReceiveDamage)
  (if _died
    (CallFunction|Die)
    (return true)
    (else
      (return false))))