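; Character component that tracks health, damage, healing and a death flag.
; ReceiveDamage spawns a blood emitter at the hit location, then ReduceHP subtracts damage, clamps at zero and returns whether HP ran out.
; Die only sets HasDied and is not called within this graph.
; ReceiveHP heals through IncreaseHP, capped at HPMax, and clears HasDied.
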(event Custom|Die
  (Variables|Default|SetHasDied true))

(event Custom|Receive%20HP
  (params (HP :type Float%20%28single-precision%29))
  (CallFunction|IncreaseHP HP)
  (Variables|Default|SetHasDied false))

(event EventBeginPlay)

(event EventTick
  (params (DeltaSeconds :type Float%20%28single-precision%29)))

(fn ReduceHP
  (params (Damage :type Float%20%28single-precision%29))
  (if (<= (- (Variables|Default|GetHP_Amount) Damage) 0.0)
    (Variables|Default|SetHP_Amount 0.0)
    (return true)
    (else
      (Variables|Default|SetHP_Amount (- (Variables|Default|GetHP_Amount) Damage))
      (return false))))

(fn IncreaseHP
  (params (HP :type Float%20%28single-precision%29))
  (if (>= (+ HP (Variables|Default|GetHP_Amount)) (Variables|Default|GetHP_Max))
    (Variables|Default|SetHP_Amount (Variables|Default|GetHP_Max))
    (else
      (Variables|Default|SetHP_Amount (+ HP (Variables|Default|GetHP_Amount)))))
  (return (>= (+ HP (Variables|Default|GetHP_Amount)) (Variables|Default|GetHP_Max))))

(fn ReceiveDamage
  (params (Damage :type Float%20%28single-precision%29) (Hit%20Location :type Vector))
  (Effects|SpawnEmitteratLocation "/Game/Assets/Particles/P_Blood.P_Blood" Hit%20Location)
  (bind _is_dead (CallFunction|ReduceHP Damage))
  (return _is_dead))